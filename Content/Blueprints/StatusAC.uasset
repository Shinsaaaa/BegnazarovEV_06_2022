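; StatusAC is a status component that tracks the hit points of its owner.
; CurrentHP starts at MaxHP on BeginPlay, and a single function subtracts a signed value to apply damage or healing, clamped between zero and MaxHP.
; Tick prints CurrentHP to screen every frame as a debug readout, using the frame's delta time as the display duration.
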(event EventBeginPlay
  (Variables|Default|SetCurrent%20HP (Variables|Default|GetMax%20HP)))

(event EventTick
  (params (DeltaSeconds :type Float%20%28single-precision%29))
  (Development|PrintString (Utilities|String|ToString(Float) (Variables|Default|GetCurrent%20HP)) true true "(R=0.000000,G=0.660000,B=1.000000,A=1.000000)" DeltaSeconds))

(fn MakeDamage/Health
  (params (Value :type Float%20%28double-precision%29))
  (Variables|Default|SetCurrent%20HP (Math|Float|Clamp(Float) (- (Variables|Default|GetCurrent%20HP) Value) 0.0 (Variables|Default|GetMax%20HP))))